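; RTS player controller that drives a BP_RTSCameraPawnBP camera pawn, cached on BeginPlay.
; Axis inputs move the pawn relative to its facing at a fixed height, with a held key doubling speed.
; Holding Pan disables movement and opens gates that let mouse input rotate yaw and clamped pitch.
; Zoom inputs step spring arm length within limits, reset inputs restore rotation or zoom, and EdgeScroll is unimplemented.
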(event EventBeginPlay
  (Utilities|FlowControl|Sequence
    (:then_0
      (Utilities|ReferenceCast))))

(event Input|ActionEvents|InputActionZoomReset
  (params (Key :type Key%20Structure :default "None"))
  ;[1 1 1] 줌 리셋
  (:Pressed
    (Variables|/Script/Engine.SpringArmComponent|SetTargetArmLength (Variables|/Game/Blueprints/BP_RTSCameraPawnBP.BP_RTSCameraPawnBP_C|GetSpringArm (Variables|References|GetCameraPawnRef)) 1.5e+03)))

(event Input|ActionEvents|InputActionZoomIn
  (params (Key :type Key%20Structure :default "None"))
  ;[1 1 1] 줌 인
  (:Pressed
    (if (< (Variables|MovementVariables|GetMinZoomLimit) (- (Variables|/Script/Engine.SpringArmComponent|GetTargetArmLength (Variables|/Game/Blueprints/BP_RTSCameraPawnBP.BP_RTSCameraPawnBP_C|GetSpringArm (Variables|References|GetCameraPawnRef))) (Variables|MovementVariables|GetZoomSpeed)))
      (Variables|/Script/Engine.SpringArmComponent|SetTargetArmLength (Variables|/Game/Blueprints/BP_RTSCameraPawnBP.BP_RTSCameraPawnBP_C|GetSpringArm (Variables|References|GetCameraPawnRef)) (- (Variables|/Script/Engine.SpringArmComponent|GetTargetArmLength (Variables|/Game/Blueprints/BP_RTSCameraPawnBP.BP_RTSCameraPawnBP_C|GetSpringArm (Variables|References|GetCameraPawnRef))) (Variables|MovementVariables|GetZoomSpeed)))
      (else
        (Variables|/Script/Engine.SpringArmComponent|SetTargetArmLength (Variables|/Game/Blueprints/BP_RTSCameraPawnBP.BP_RTSCameraPawnBP_C|GetSpringArm (Variables|References|GetCameraPawnRef)) (Variables|MovementVariables|GetMinZoomLimit))))))

(event Input|ActionEvents|InputActionPanReset
  (params (Key :type Key%20Structure :default "None"))
  ;[1 1 1] 팬 리셋
  (:Pressed
    (Transformation|SetActorRotation (Variables|References|GetCameraPawnRef) (Math|Rotator|MakeRotator (.Roll (Math|Rotator|BreakRotator (Transformation|GetActorRotation (Variables|References|GetCameraPawnRef)))) 0.0 0.0))))

(event Input|ActionEvents|InputActionPan
  (params (Key :type Key%20Structure :default "None"))
  (bind _camerapawnref (Variables|References|GetCameraPawnRef))
  (bind _returnvalue (Transformation|GetActorRotation _camerapawnref))
  (bind (_roll _pitch _yaw) (Math|Rotator|BreakRotator _returnvalue))
  (:Pressed
    (Variables|Bool|SetDisableCanMovement true)
    ;[1 1 1] 팬 Y
    (Utilities|FlowControl|Gate true) ; enters at Open
  )
  (:Released
    (Variables|Bool|SetDisableCanMovement false)
    (Utilities|FlowControl|Gate true) ; enters at Close
  ))

(event Input|ActionEvents|InputActionPan
  (params (Key :type Key%20Structure :default "None"))
  (bind _camerapawnref (Variables|References|GetCameraPawnRef))
  (bind _returnvalue (Transformation|GetActorRotation _camerapawnref))
  (bind (_roll _pitch _yaw) (Math|Rotator|BreakRotator _returnvalue))
  (:Pressed
    (Variables|Bool|SetDisableCanMovement true)
    ;[1 1 1] 팬 X (게이트 대신 bool변수 만들고 branch로 작성가능)
    (Utilities|FlowControl|Gate true) ; enters at Open
  )
  (:Released
    (Variables|Bool|SetDisableCanMovement false)
    (Utilities|FlowControl|Gate true) ; enters at Close
  ))

(event Input|ActionEvents|InputActionZoomOut
  (params (Key :type Key%20Structure :default "None"))
  ;[1 1 1] 줌 아웃
  (:Pressed
    (if (> (Variables|MovementVariables|GetMaxZoomLimit) (+ (Variables|/Script/Engine.SpringArmComponent|GetTargetArmLength (Variables|/Game/Blueprints/BP_RTSCameraPawnBP.BP_RTSCameraPawnBP_C|GetSpringArm (Variables|References|GetCameraPawnRef))) (Variables|MovementVariables|GetZoomSpeed)))
      (Variables|/Script/Engine.SpringArmComponent|SetTargetArmLength (Variables|/Game/Blueprints/BP_RTSCameraPawnBP.BP_RTSCameraPawnBP_C|GetSpringArm (Variables|References|GetCameraPawnRef)) (+ (Variables|/Script/Engine.SpringArmComponent|GetTargetArmLength (Variables|/Game/Blueprints/BP_RTSCameraPawnBP.BP_RTSCameraPawnBP_C|GetSpringArm (Variables|References|GetCameraPawnRef))) (Variables|MovementVariables|GetZoomSpeed)))
      (else
        (Variables|/Script/Engine.SpringArmComponent|SetTargetArmLength (Variables|/Game/Blueprints/BP_RTSCameraPawnBP.BP_RTSCameraPawnBP_C|GetSpringArm (Variables|References|GetCameraPawnRef)) (Variables|MovementVariables|GetMaxZoomLimit))))))

(event Input|ActionEvents|InputActionSpeedModifier
  (params (Key :type Key%20Structure :default "None"))
  (:Pressed
    (Variables|MovementVariables|SetMovementSpeedModifier 2.0))
  (:Released
    (Variables|MovementVariables|SetMovementSpeedModifier 1.0)))

(event Input|AxisEvents|InputAxisMoveForward
  (params (AxisValue :type Float%20%28single-precision%29))
  (Variables|Default|SetForwardValue AxisValue)
  (if (not (Variables|Bool|GetDisableCanMovement))
    (Transformation|SetActorLocation (Variables|References|GetCameraPawnRef) (Math|Vector|MakeVector (.X (Math|Vector|BreakVector (Math|Transform|TransformLocation (Transformation|GetActorTransform (Variables|References|GetCameraPawnRef)) (Math|Vector|MakeVector (* (Variables|Default|GetForwardValue) (* (Variables|MovementVariables|GetDefaultMovementSpeed) (Variables|MovementVariables|GetMovementSpeedModifier))) 0.0 0.0)))) (.Y (Math|Vector|BreakVector (Math|Transform|TransformLocation (Transformation|GetActorTransform (Variables|References|GetCameraPawnRef)) (Math|Vector|MakeVector (* (Variables|Default|GetForwardValue) (* (Variables|MovementVariables|GetDefaultMovementSpeed) (Variables|MovementVariables|GetMovementSpeedModifier))) 0.0 0.0)))) 2e+02) true false)))

(event Input|AxisEvents|InputAxisMoveRight
  (params (AxisValue :type Float%20%28single-precision%29))
  (Variables|Default|SetRightValue AxisValue)
  (if (not (Variables|Bool|GetDisableCanMovement))
    (Transformation|SetActorLocation (Variables|References|GetCameraPawnRef) (Math|Vector|MakeVector (.X (Math|Vector|BreakVector (Math|Transform|TransformLocation (Transformation|GetActorTransform (Variables|References|GetCameraPawnRef)) (Math|Vector|MakeVector 0.0 (* (Variables|Default|GetRightValue) (* (Variables|MovementVariables|GetDefaultMovementSpeed) (Variables|MovementVariables|GetMovementSpeedModifier))) 0.0)))) (.Y (Math|Vector|BreakVector (Math|Transform|TransformLocation (Transformation|GetActorTransform (Variables|References|GetCameraPawnRef)) (Math|Vector|MakeVector 0.0 (* (Variables|Default|GetRightValue) (* (Variables|MovementVariables|GetDefaultMovementSpeed) (Variables|MovementVariables|GetMovementSpeedModifier))) 0.0)))) 2e+02) true false)))

(event Input|MouseEvents|MouseX
  (params (AxisValue :type Float%20%28single-precision%29))
  (bind _camerapawnref (Variables|References|GetCameraPawnRef))
  (bind _returnvalue (Transformation|GetActorRotation _camerapawnref))
  (bind (_roll _pitch _yaw) (Math|Rotator|BreakRotator _returnvalue))
  ;[1 1 1] 팬 X (게이트 대신 bool변수 만들고 branch로 작성가능)
  (Utilities|FlowControl|Gate true
    (:Exit
      (Transformation|SetActorRotation (Variables|References|GetCameraPawnRef) (Math|Rotator|MakeRotator _roll _pitch (+ _yaw (* AxisValue (Variables|MovementVariables|GetPanSpeed))))))))

(event Input|MouseEvents|MouseY
  (params (AxisValue :type Float%20%28single-precision%29))
  (bind _camerapawnref (Variables|References|GetCameraPawnRef))
  (bind _returnvalue (Transformation|GetActorRotation _camerapawnref))
  (bind (_roll _pitch _yaw) (Math|Rotator|BreakRotator _returnvalue))
  ;[1 1 1] 팬 Y
  (Utilities|FlowControl|Gate true
    (:Exit
      (Transformation|SetActorRotation (Variables|References|GetCameraPawnRef) (Math|Rotator|MakeRotator _roll (Math|Float|Clamp(Float) (+ _pitch (* AxisValue (Variables|MovementVariables|GetPanSpeed))) -22.5 45.0) _yaw)))))

(fn ConstructionScript)